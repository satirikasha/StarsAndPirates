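; World manager that streams a grid of world segments around the one most recently entered, starting from a pre-assigned initial segment.
; Each segment's entered event re-centers the grid, destroying segments outside the surrounding 3x3 block and spawning missing cells.
; New segment classes come from the FlyingGameMode's SegmentProvider and spawn at the manager's transform, receiving their grid coordinates and an event binding back to the manager.
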(event EventBeginPlay
  (CallFunction|OnEnteredSegment (Variables|Default|GetInitialWorldSegment)))

(event EventActorBeginOverlap
  (params (OtherActor :type Actor%20Object%20Reference)))

(event EventTick
  (params (DeltaSeconds :type Float%20%28single-precision%29)))

(fn ConstructionScript
  (bind _initialworldsegment (Variables|Default|GetInitialWorldSegment))
  (EventDispatchers|BindEventtoOnEnteredSegment _initialworldsegment (EventDispatchers|CreateEvent :!event OnEnteredSegment))
  (Utilities|Array|Add (Variables|Default|GetGeneratedSegments) _initialworldsegment)
  (Utilities|Array|Add (Variables|Default|GetSpawnedSegments) _initialworldsegment))

(fn OnEnteredSegment
  (params (Segment :type World%20Segment%20Object%20Reference))
  (bind _output_get (Variables|Default|SetCurrentWorldSegment Segment))
  (CallFunction|RemoveUnusedSegments (Variables|/Game/Blueprints/World/WorldSegment.WorldSegment_C|GetWorldX _output_get) (Variables|/Game/Blueprints/World/WorldSegment.WorldSegment_C|GetWorldY _output_get))
  (for _index (range -1 1)
    (for _index_2 (range -1 1)
      (bind _result (CallFunction|IsSegmentSpawned (+ _index (Variables|/Game/Blueprints/World/WorldSegment.WorldSegment_C|GetWorldX _output_get)) (+ _index_2 (Variables|/Game/Blueprints/World/WorldSegment.WorldSegment_C|GetWorldY _output_get))))
      (if (not _result)
        (bind _class (Default|GetSegment (Variables|/Game/Blueprints/FlyingGameMode.FlyingGameMode_C|GetSegmentProvider (.AsFlying%20Game%20Mode (Utilities|Casting|CastToFlyingGameMode (Game|GetGameMode))))))
        (bind _returnvalue (Game|SpawnActorfromClass _class (Transformation|GetActorTransform) "AlwaysSpawn" 0 (+ _index (Variables|/Game/Blueprints/World/WorldSegment.WorldSegment_C|GetWorldX _output_get)) (+ _index_2 (Variables|/Game/Blueprints/World/WorldSegment.WorldSegment_C|GetWorldY _output_get))))
        (EventDispatchers|BindEventtoOnEnteredSegment _returnvalue (EventDispatchers|CreateEvent :!event OnEnteredSegment))
        (Utilities|Array|Add (Variables|Default|GetSpawnedSegments) _returnvalue)))))

(fn RemoveUnusedSegments
  (params (WorldX :type Integer) (WorldY :type Integer))
  (for _array_element (Variables|Default|GetSpawnedSegments)
    (if (or (> (Math|Integer|Absolute(Integer) (- (Variables|/Game/Blueprints/World/WorldSegment.WorldSegment_C|GetWorldX _array_element) WorldX)) 1) (> (Math|Integer|Absolute(Integer) (- (Variables|/Game/Blueprints/World/WorldSegment.WorldSegment_C|GetWorldY _array_element) WorldY)) 1))
      (Actor|DestroyActor _array_element)
      (Utilities|Array|Add (LocalVariables|GetActorsToRemove) _array_element)))
  (for _array_element_2 (LocalVariables|GetActorsToRemove)
    (Utilities|Array|RemoveItem (Variables|Default|GetSpawnedSegments) _array_element_2)))

(fn IsSegmentSpawned
  (params (WorldX :type Integer) (WorldY :type Integer))
  (bind _array_element (Utilities|Array|ForEachLoopwithBreak (Variables|Default|GetSpawnedSegments) :!label _label)
    (:LoopBody
      (if (and (== (Variables|/Game/Blueprints/World/WorldSegment.WorldSegment_C|GetWorldX _array_element) WorldX) (== (Variables|/Game/Blueprints/World/WorldSegment.WorldSegment_C|GetWorldY _array_element) WorldY))
        (goto _label Break)))
    (:Completed
      (return (and (== (Variables|/Game/Blueprints/World/WorldSegment.WorldSegment_C|GetWorldX _array_element) WorldX) (== (Variables|/Game/Blueprints/World/WorldSegment.WorldSegment_C|GetWorldY _array_element) WorldY))))))