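; WorldSegment is one grid cell of the game world that detects when a SpaceShip enters it.
; The construction script reads WorldSegmentSize from the WorldParameters collection, sizes SegmentVolume to match, and places the actor by its WorldX/WorldY grid coordinates.
; SpaceShip overlaps fire the OnEnteredSegment dispatcher and print the coordinates.
; GetRandomLocation returns a random Z-flattened point within the box extent, centered on zero rather than the actor's location.
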(event `self.ReceiveBeginPlay`)

(event `self.ReceiveActorBeginOverlap`
  (params (OtherActor :type "Actor Object Reference")))

(event `self.ReceiveTick`
  (params (DeltaSeconds :type "Float (single-precision)")))

(event `self.SegmentVolume.OnComponentBeginOverlap`
  (params (OtherActor :type "Actor Object Reference") (OtherComp :type "PrimitiveComponent Object Reference") (OtherBodyIndex :type Integer) (bFromSweep :type Boolean) (SweepResult :type "HitResult Structure (by ref)"))
  (cast `/Game/Blueprints/Ship/SpaceShip` OtherActor)
  (`self.OnEnteredSegment` self)
  (`KismetSystemLibrary.PrintString` (`KismetStringLibrary.Concat_StrStr` "Entered Segment: " (`KismetStringLibrary.Conv_IntToString` (`self.WorldX`)) " " (`KismetStringLibrary.Conv_IntToString` (`self.WorldY`)))))

(fn `GetRandomLocation`
  (returns (Location :type "Vector Structure"))
  (return (* (`KismetMathLibrary.RandomPointInBoundingBox` (`KismetMathLibrary.MakeVector` 0.0) (`BoxComponent.BoxExtent` (`self.SegmentVolume`))) (1.0 1.0 0.0))))

(fn `UserConstructionScript`
  (bind _returnvalue (`KismetMaterialLibrary.GetScalarParameterValue` "/Game/Blueprints/Data/WorldParameters.WorldParameters" "WorldSegmentSize"))
  (bind _output_get (set `self.WorldSegmentSize` _returnvalue))
  (bind _returnvalue_2 (/ _output_get 2.0))
  (`BoxComponent.SetBoxExtent` (`self.SegmentVolume`) (`KismetMathLibrary.MakeVector` _returnvalue_2 _returnvalue_2 500.0) true)
  (`self.K2_SetActorLocation` (`KismetMathLibrary.MakeVector` (* (`self.WorldX`) (`self.WorldSegmentSize`)) (* (`self.WorldY`) (`self.WorldSegmentSize`))) false true))