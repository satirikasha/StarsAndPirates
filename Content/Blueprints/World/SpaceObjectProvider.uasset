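; SpaceObjectProvider hands out space objects by weighted random choice from the SpaceObjectGenerationData table.
; Its construction script copies table rows into GenerationData and totals their probabilities.
; GetSpaceObject accumulates weights until one passes a random threshold, re-rolled at each entry, then returns that object.
; Positive count limits decrement per pick; exhausted entries drop to zero weight and leave the total, while non-positive limits stay unchanged.
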(event EventActorBeginOverlap
  (params (OtherActor :type Actor%20Object%20Reference)))

(event EventTick
  (params (DeltaSeconds :type Float%20%28single-precision%29)))

(fn ConstructionScript
  (bind _outrownames (DataTable|GetDataTableRowNames "/Game/Blueprints/Data/SpaceObjectGenerationData.SpaceObjectGenerationData"))
  (for _array_element _outrownames
    (bind _returnvalue (Utilities|GetDataTableRow "/Game/Blueprints/Data/SpaceObjectGenerationData.SpaceObjectGenerationData" _array_element)
      (:then
        (Variables|Default|SetUnitProbability (+ (.Probability (Utilities|Struct|BreakSpaceObjectGenerationRecord _returnvalue)) (Variables|Default|GetUnitProbability)))
        (Utilities|Array|Add (Variables|Default|GetGenerationData) _returnvalue)))))

(fn GetSpaceObject
  (bind (_array_element _array_index) (Utilities|Array|ForEachLoopwithBreak (Variables|Default|GetGenerationData) :!label _label)
    (:LoopBody
      (LocalVariables|SetCurrentProbability (+ (.Probability (Utilities|Struct|BreakSpaceObjectGenerationRecord _array_element)) (LocalVariables|GetCurrentProbability)))
      (if (>= (LocalVariables|GetCurrentProbability) (* (Math|Random|RandomFloat) (Variables|Default|GetUnitProbability)))
        (LocalVariables|SetResultIndex _array_index)
        (goto _label Break)))
    (:Completed
      (if (> (.CountLimit (Utilities|Struct|BreakSpaceObjectGenerationRecord (Utilities|Array|Get(acopy) (Variables|Default|GetGenerationData) (LocalVariables|GetResultIndex)))) 0)
        (Variables|Default|SetUnitProbability (- (Variables|Default|GetUnitProbability) (Math|Float|SelectFloat 0.0 (.Probability (Utilities|Struct|BreakSpaceObjectGenerationRecord (Utilities|Array|Get(acopy) (Variables|Default|GetGenerationData) (LocalVariables|GetResultIndex)))) (> (- (.CountLimit (Utilities|Struct|BreakSpaceObjectGenerationRecord (Utilities|Array|Get(acopy) (Variables|Default|GetGenerationData) (LocalVariables|GetResultIndex)))) 1) 0))))
        (Utilities|Array|SetArrayElem (Variables|Default|GetGenerationData) (LocalVariables|GetResultIndex) (Utilities|Struct|MakeSpaceObjectGenerationRecord (.SpaceObject (Utilities|Struct|BreakSpaceObjectGenerationRecord (Utilities|Array|Get(acopy) (Variables|Default|GetGenerationData) (LocalVariables|GetResultIndex)))) (Math|Float|SelectFloat (.Probability (Utilities|Struct|BreakSpaceObjectGenerationRecord (Utilities|Array|Get(acopy) (Variables|Default|GetGenerationData) (LocalVariables|GetResultIndex)))) 0.0 (> (- (.CountLimit (Utilities|Struct|BreakSpaceObjectGenerationRecord (Utilities|Array|Get(acopy) (Variables|Default|GetGenerationData) (LocalVariables|GetResultIndex)))) 1) 0)) (- (.CountLimit (Utilities|Struct|BreakSpaceObjectGenerationRecord (Utilities|Array|Get(acopy) (Variables|Default|GetGenerationData) (LocalVariables|GetResultIndex)))) 1))))
      (return (.SpaceObject (Utilities|Struct|BreakSpaceObjectGenerationRecord (Utilities|Array|Get(acopy) (Variables|Default|GetGenerationData) (LocalVariables|GetResultIndex))))))))