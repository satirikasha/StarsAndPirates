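; Behavior tree task that picks a random nearby location for the AI-controlled pawn and stores it in the TargetLocation blackboard key.
; It flattens a random unit vector onto the horizontal plane, normalizes it, scales it by a random distance up to 1000 units and adds it to the pawn's location.
; It prints a debug string and finishes successfully at once, with no navmesh or reachability check.
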(event `self.ReceiveExecuteAI`
  (params (OwnerController :type "AIController Object Reference") (ControlledPawn :type "Pawn Object Reference"))
  (`BTFunctionLibrary.SetBlackboardValueAsVector` (`self.TargetLocation`) (+ (`Actor.K2_GetActorLocation` ControlledPawn) (* (`KismetMathLibrary.Normal` (* (`KismetMathLibrary.RandomUnitVector`) (1.0 1.0 0.0))) (* (`KismetMathLibrary.RandomFloat`) 1000.0))))
  (`KismetSystemLibrary.PrintString` "ChooseRandom")
  (`self.FinishExecute` true))