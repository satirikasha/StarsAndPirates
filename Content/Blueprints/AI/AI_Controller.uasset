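; AI controller that runs a behavior tree and flies a SpaceShip pawn to target locations.
; FlyTo stores the target and returns a TaskResult, which is notified within the acceptable radius.
; Each tick, sphere traces sweep alternately left and right in widening yaw steps to find a clear heading around obstacles.
; Dot products and a steer curve convert that heading into turn and throttle input, with debug drawing throughout.
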(event EventBeginPlay
  (AI|RunBehaviorTree "/Game/Blueprints/AI/AI_BehaviorTree.AI_BehaviorTree"))

(event EventTick
  (params (DeltaSeconds :type Float%20%28single-precision%29))
  (CallFunction|TickFlyto 0.0))

(fn ConstructionScript)

(fn Flyto
  (params (Location :type Vector) (AcceptableRadius :type Float%20%28single-precision%29))
  (Variables|Default|SetAcceptableRadius AcceptableRadius)
  (Variables|Default|SetTargetLocation Location)
  (Variables|Default|SetIsFlyToInProgress true)
  (bind _returnvalue (Game|ConstructObjectfromClass "/Game/Blueprints/AI/TaskResult.TaskResult_C" self))
  (bind _output_get (Variables|Default|SetCurrentTaskResult _returnvalue))
  (return _output_get))

(fn TickFlyto
  (params (DeltaTime :type Float%20%28single-precision%29))
  (if (Variables|Default|GetIsFlyToInProgress)
    (CallFunction|CalculateCurrentTargetLocation)
    (CallFunction|NavigatetoCurrentTargetLocation)
    (CallFunction|CheckDistancetoTargetlocation)))

(fn CalculateCurrentTargetLocation
  (bind _returnvalue (Pawn|GetControlledPawn))
  (bind _targetlocation (Variables|Default|GetTargetLocation))
  (bind _returnvalue_2 (Transformation|GetActorLocation _returnvalue))
  (Rendering|Debug|DrawDebugSphere _targetlocation 5e+01 12 "(R=1.000000,G=0.812809,B=0.000000,A=1.000000)" 0.0)
  (Utilities|FlowControl|ForLoopwithBreak 0 15 :!label _label
    (:LoopBody
      (bind _returnvalue_3 (Collision|SphereTraceForObjects _returnvalue_2 (+ _returnvalue_2 (Math|Vector|RotateVectorAroundAxis (* (Math|Vector|Normalize (- _targetlocation _returnvalue_2)) 1e+03) (LocalVariables|GetRotationAngle) "0, 0,1.000000")) 1e+02 (Utilities|Array|MakeArray "ObjectTypeQuery1" "ObjectTypeQuery4") false (Utilities|Array|MakeArray _returnvalue) "ForOneFrame"))
      (if _returnvalue_3
        (Utilities|FlowControl|FlipFlop
          (:A
            (LocalVariables|SetRotationAngle (+ (Math|Float|Absolute(Float) (LocalVariables|GetRotationAngle)) 5.0)))
          (:B
            (LocalVariables|SetRotationAngle (* -1 (+ (Math|Float|Absolute(Float) (LocalVariables|GetRotationAngle)) 5.0)))))
        (else
          (goto _label Break))))
    (:Completed
      (bind _output_get (Variables|Default|SetCurrentTargetLocation (+ _returnvalue_2 (Math|Vector|RotateVectorAroundAxis (* (Math|Vector|Normalize (- _targetlocation _returnvalue_2)) 1e+03) (LocalVariables|GetRotationAngle) "0, 0,1.000000"))))
      (Rendering|Debug|DrawDebugSphere _output_get 5e+01 12 "(R=0.000000,G=0.470675,B=1.000000,A=1.000000)" 0.0))))

(fn NavigatetoCurrentTargetLocation
  (bind _asspace_ship (Utilities|Casting|CastToSpaceShip (Pawn|GetControlledPawn)))
  (Variables|/Game/Blueprints/Ship/SpaceShip.SpaceShip_C|SetTurnAxis _asspace_ship (* (Math|Float|Sign(Float) (* -1 (Math|Vector|DotProduct (Math|Vector|Normalize (- (Variables|Default|GetCurrentTargetLocation) (Transformation|GetActorLocation _asspace_ship))) (Math|Vector|Normalize (Math|Vector|CrossProduct (Math|Vector|GetForwardVector (Variables|/Game/Blueprints/Ship/SpaceShip.SpaceShip_C|GetDirection _asspace_ship)) "0, 0,1.000000"))))) (Math|Curves|GetFloatValue (Variables|Default|GetSteerCurve) (- 1.0 (/ (+ (Math|Vector|DotProduct (Math|Vector|Normalize (- (Variables|Default|GetCurrentTargetLocation) (Transformation|GetActorLocation _asspace_ship))) (Math|Vector|GetForwardVector (Variables|/Game/Blueprints/Ship/SpaceShip.SpaceShip_C|GetDirection _asspace_ship))) 1.0) 2.0)))))
  (Variables|/Game/Blueprints/Ship/SpaceShip.SpaceShip_C|SetThrottleAxis _asspace_ship (Math|Float|Clamp(Float) (Math|Vector|DotProduct (Math|Vector|Normalize (- (Variables|Default|GetCurrentTargetLocation) (Transformation|GetActorLocation _asspace_ship))) (Math|Vector|GetForwardVector (Variables|/Game/Blueprints/Ship/SpaceShip.SpaceShip_C|GetDirection _asspace_ship))))))

(fn CheckDistancetoTargetlocation
  (if (<= (Math|Vector|VectorLength (- (Variables|Default|GetTargetLocation) (Transformation|GetActorLocation (Pawn|GetControlledPawn)))) (Variables|Default|GetAcceptableRadius))
    (Default|CallOnTaskFinished (Variables|Default|GetCurrentTaskResult))))