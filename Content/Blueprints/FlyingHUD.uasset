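; FlyingHUD is the HUD class that manages the game HUD, pause menu and inventory widgets.
; It creates all three hidden at BeginPlay, caches the first PostProcessVolume, then shows the game HUD.
; PauseGame and OpenInventory toggle game pause or jump between menus through SwitchCurrentHUD.
; SwitchCurrentHUD swaps visibility, sets the mouse cursor and depth-of-field override for menus, and calls Refresh on IRefreshable widgets.
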(event `self.ReceiveBeginPlay`
  (`|ExecutionSequence`
    (:`then_0`
      (bind _returnvalue (`|CreateWidget` "/Game/Blueprints/UI/GameHUD.GameHUD_C"))
      (bind _output_get (set `self.GameHUD` _returnvalue))
      (`UserWidget.AddToViewport` _output_get 0)
      (`Widget.SetVisibility` _output_get "Hidden"))
    (:`then_1`
      (bind _returnvalue_2 (`|CreateWidget` "/Game/Blueprints/UI/PauseMenu.PauseMenu_C"))
      (bind _output_get_2 (set `self.PauseMenu` _returnvalue_2))
      (`UserWidget.AddToViewport` _output_get_2 0)
      (`Widget.SetVisibility` _output_get_2 "Hidden"))
    (:`then_2`
      (bind _returnvalue_3 (`|CreateWidget` "/Game/Blueprints/UI/GameInventory.GameInventory_C"))
      (bind _output_get_3 (set `self.GameInventoty` _returnvalue_3))
      (`UserWidget.AddToViewport` _output_get_3 0)
      (`Widget.SetVisibility` _output_get_3 "Hidden"))
    (:`then_3`
      (bind _outactors (`GameplayStatics.GetAllActorsOfClass` "/Script/Engine.PostProcessVolume"))
      (set `self.GlobalPostProcess` (`KismetArrayLibrary.Array_Get` _outactors))
      (`self.SwitchCurrentHUD` (`self.GameHUD`)))))

(event `self.ReceiveActorBeginOverlap`
  (params (OtherActor :type "Actor Object Reference")))

(event `self.ReceiveTick`
  (params (DeltaSeconds :type "Float (single-precision)")))

(fn `OpenInventory`
  (if (or (== (`self.CurrentHUD`) (`self.GameInventoty`)) (== (`self.CurrentHUD`) (`self.GameHUD`)))
    (`GameplayStatics.SetGamePaused` (not (`GameplayStatics.IsGamePaused`)))
    (if (`GameplayStatics.IsGamePaused`)
      (`self.SwitchCurrentHUD` (`self.GameInventoty`))
      (else
        (`self.SwitchCurrentHUD` (`self.GameHUD`))))
    (else
      (`self.SwitchCurrentHUD` (`self.GameInventoty`)))))

(fn `PauseGame`
  (if (or (== (`self.CurrentHUD`) (`self.PauseMenu`)) (== (`self.CurrentHUD`) (`self.GameHUD`)))
    (`GameplayStatics.SetGamePaused` (not (`GameplayStatics.IsGamePaused`)))
    (if (`GameplayStatics.IsGamePaused`)
      (`self.SwitchCurrentHUD` (`self.PauseMenu`))
      (else
        (`self.SwitchCurrentHUD` (`self.GameHUD`))))
    (else
      (`self.SwitchCurrentHUD` (`self.PauseMenu`)))))

(fn `SwitchCurrentHUD`
  (params (NewHUD :type "Widget Object Reference"))
  (bind _returnvalue (`GameplayStatics.GetPlayerController` 0))
  (bind _currenthud (`self.CurrentHUD`))
  (bind _returnvalue_2 (`PlayerController.GetHUD` _returnvalue))
  (`|ExecutionSequence`
    (:`then_0`
      (`/Engine/EditorBlueprintResources/StandardMacros.IsValid` _currenthud
        (:`Is Valid`
          (`Widget.SetVisibility` _currenthud "Hidden"))))
    (:`then_1`
      (bind _output_get (set `self.CurrentHUD` NewHUD))
      (`Widget.SetVisibility` _output_get "Visible"))
    (:`then_2`
      (if (== NewHUD (`self.GameHUD`))
        (set `PlayerController.bShowMouseCursor` false _returnvalue)
        (bind _asflying_hud (cast `/Game/Blueprints/FlyingHUD` _returnvalue_2))
        (setmembers `PostProcessSettings` :`StructRef` (`PostProcessVolume.Settings` (`/Game/Blueprints/FlyingHUD.GlobalPostProcess` _asflying_hud)) :`bOverride_DepthOfFieldMethod` false)
        (else
          (set `PlayerController.bShowMouseCursor` true _returnvalue)
          (bind _asflying_hud_2 (cast `/Game/Blueprints/FlyingHUD` _returnvalue_2))
          (setmembers `PostProcessSettings` :`StructRef` (`PostProcessVolume.Settings` (`/Game/Blueprints/FlyingHUD.GlobalPostProcess` _asflying_hud_2)) :`bOverride_DepthOfFieldMethod` true))))
    (:`then_3`
      (bind _asirefreshable (cast `/Game/Blueprints/UI/Tools/IRefreshable` NewHUD))
      (`/Game/Blueprints/UI/Tools/IRefreshable.Refresh` _asirefreshable))))

(fn `UserConstructionScript`)