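; Generator actor that supplies energy to the SpaceShip that owns it.
; On BeginPlay it casts its owner to SpaceShip and caches the reference.
; Each Tick, while that ship is valid and not dead, it passes EnergyCreation scaled by delta time to AffectEnergy, negated so production counts as negative consumption.
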(event `self.ReceiveBeginPlay`
  (bind _asspace_ship (cast `/Game/Blueprints/Ship/SpaceShip` (`self.GetOwner`)))
  (set `self.SpaceShip` _asspace_ship))

(event `self.ReceiveActorBeginOverlap`
  (params (OtherActor :type "Actor Object Reference")))

(event `self.ReceiveTick`
  (params (DeltaSeconds :type "Float (single-precision)"))
  (bind _spaceship (`self.SpaceShip`))
  (`/Engine/EditorBlueprintResources/StandardMacros.IsValid` _spaceship
    (:`Is Valid`
      (if (not (`/Game/Blueprints/Ship/SpaceShip.IsDead` _spaceship))
        (`/Game/Blueprints/Ship/SpaceShip.AffectEnergy` _spaceship (* DeltaSeconds (`self.EnergyCreation`) -1.0))))))

(fn `UserConstructionScript`)