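; Ship weapon that auto-fires projectiles while the trigger is held.
; PullTrigger fires once immediately through a DoOnce, then starts a looping ReloadTime timer; ReleaseTrigger clears the timer and resets the gate, so re-pulling fires without waiting.
; Each shot spawns at the Arrow's location flattened to Z=0 with its rotation, inherits the owning SpaceShip's planar velocity, and gets a limited life span.
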(event `PullTrigger`
  (`/Engine/EditorBlueprintResources/StandardMacros.DoOnce` false :!label _label
    (:`Completed`
      (`self.Fire`)
      (bind _returnvalue (`KismetSystemLibrary.K2_SetTimerDelegate` (delegate `Fire`) (`self.ReloadTime`) true))
      (set `self.ReloadingTimerHandle` _returnvalue))))

(event `ReleaseTrigger`
  (`KismetSystemLibrary.K2_ClearTimerHandle` (`self.ReloadingTimerHandle`))
  (goto _label :!via `Reset`))

(event `Fire`
  (bind _arrow (`self.Arrow`))
  (bind _returnvalue (`|SpawnActorFromClass` (`self.Projectile`) (`KismetMathLibrary.MakeTransform` (* (`SceneComponent.K2_GetComponentLocation` _arrow) (1.0 1.0 0.0)) (`SceneComponent.K2_GetComponentRotation` _arrow)) "Undefined" "OverrideRootScale" null (`/Game/Blueprints/Ship/SpaceShip.GetPlanarVelocity` (cast `/Game/Blueprints/Ship/SpaceShip` (`self.GetOwner`) :!pure true))))
  (`self.SetLifeSpan` _returnvalue (`self.InitialLifeSpan`)))

(fn `UserConstructionScript`)