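; Ship engine actor that turns throttle input into thrust for the SpaceShip that owns it.
; RecieveThrottle checks the ship's Energy against a cost scaled by throttle, DeltaTime and EnergyConsumption.
; With enough energy, it applies throttle-scaled EngineForce to the supplied body, sets the particle system's Throttle parameter and passes the cost to AffectEnergy.
; Otherwise it applies no force and zeroes the particle throttle.
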(event `self.ReceiveBeginPlay`
  (`parent.ReceiveBeginPlay`))

(event `self.ReceiveActorBeginOverlap`
  (params (OtherActor :type "Actor Object Reference")))

(event `self.ReceiveTick`
  (params (DeltaSeconds :type "Float (single-precision)")))

(fn `RecieveThrottle`
  (params (Throttle :type "Float (double-precision)") (Body :type "PrimitiveComponent Object Reference") (ForceDirection :type "Vector Structure") (DeltaTime :type "Float (double-precision)"))
  (bind _particlesystem (`self.ParticleSystem`))
  (bind _returnvalue (* Throttle DeltaTime (`self.EnergyConsumption`)))
  (bind _asspace_ship (cast `/Game/Blueprints/Ship/SpaceShip` (`self.GetOwner`)))
  (if (>= (`/Game/Blueprints/Ship/SpaceShip.Energy` _asspace_ship) _returnvalue)
    (`PrimitiveComponent.AddForce` Body (* ForceDirection (* Throttle (`self.EngineForce`))) "None" false)
    (`ParticleSystemComponent.SetFloatParameter` _particlesystem "Throttle" Throttle)
    (`/Game/Blueprints/Ship/SpaceShip.AffectEnergy` _asspace_ship _returnvalue)
    (else
      (`ParticleSystemComponent.SetFloatParameter` _particlesystem "Throttle" 0.0))))

(fn `UserConstructionScript`
  (`parent.UserConstructionScript`))