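; Raider ship Blueprint, a child ship class that defines the default loadout for its sockets.
; Its SetSocketsDefaultItems event loops over SocketSlots and switches on each slot's socket type.
; Engine, Weapon and Tool slots receive items looked up by row name in the ItemData table: a Union engine, Raider weapon and Raider generator.
; The construction script only calls its parent.
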(event `self.ReceiveBeginPlay`
  (`parent.ReceiveBeginPlay`))

(event `self.ReceiveActorBeginOverlap`
  (params (OtherActor :type "Actor Object Reference")))

(event `self.ReceiveTick`
  (params (DeltaSeconds :type "Float (single-precision)"))
  (`parent.ReceiveTick` 0.0))

(event `self.SetSocketsDefaultItems`
  (for _array_element (`self.SocketSlots`)
    (switch `/Game/Blueprints/Data/ItemType` (`/Game/Blueprints/Ship/SocketSlot.SocketType` _array_element)
      (:`NewEnumerator1`
        (bind _returnvalue (`|GetDataTableRow` "/Game/Blueprints/Data/ItemData.ItemData" "UnionEngine_01")
          (:`then`
            (`/Game/Blueprints/Ship/SocketSlot.SetItem` _array_element _returnvalue))))
      (:`NewEnumerator2`
        (bind _returnvalue_2 (`|GetDataTableRow` "/Game/Blueprints/Data/ItemData.ItemData" "RaiderWeapon_01")
          (:`then`
            (`/Game/Blueprints/Ship/SocketSlot.SetItem` _array_element _returnvalue_2))))
      (:`NewEnumerator3`
        (bind _returnvalue_3 (`|GetDataTableRow` "/Game/Blueprints/Data/ItemData.ItemData" "RaiderGenerator_01")
          (:`then`
            (`/Game/Blueprints/Ship/SocketSlot.SetItem` _array_element _returnvalue_3)))))))

(fn `UserConstructionScript`
  (`parent.UserConstructionScript`))