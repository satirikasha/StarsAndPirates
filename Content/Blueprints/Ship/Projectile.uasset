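; Ship projectile that inherits launcher velocity along its forward axis and has a slightly randomized lifespan.
; On overlap it damages any IDamageable actor and destroys itself, ignoring the instigating ship and its ShipParts for the first second.
; When destroyed it spawns either a hit effect or an expiry effect, depending on whether a hit ended it.
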(event `self.ReceiveBeginPlay`
  (`KismetSystemLibrary.Delay` 1.0)
  (set `self.CanHitParent` true))

(event `self.Sphere.OnComponentBeginOverlap`
  (params (OtherActor :type "Actor Object Reference") (OtherComp :type "PrimitiveComponent Object Reference") (OtherBodyIndex :type Integer) (bFromSweep :type Boolean) (SweepResult :type "HitResult Structure (by ref)"))
  (if (and (`KismetSystemLibrary.DoesImplementInterface` OtherActor "/Game/Blueprints/Ship/IDamageable.IDamageable_C") (or (`self.CanHitParent`) (not (`self.BelongsToInstigator` OtherActor))))
    (`GameplayStatics.ApplyDamage` OtherActor (`self.Damage`) null self (`self.DamageType`))
    (set `self.DestroyedByHit` true)
    (`self.K2_DestroyActor`)))

(event `self.ReceiveDestroyed`
  (`|SpawnActorFromClass` (castclass `Actor` (`KismetMathLibrary.SelectClass` (`self.HitEffect`) (`self.DestroyedEffect`) (`self.DestroyedByHit`)) :!pure true) (`self.GetTransform`) "AlwaysSpawn" "OverrideRootScale"))

(fn `BelongsToInstigator`
  (params (TestActor :type "Actor Object Reference"))
  (returns (Result :type Boolean))
  (bind _returnvalue (`self.GetInstigator`))
  (bind _asspace_ship (cast `/Game/Blueprints/Ship/SpaceShip` TestActor)
    (:`then`
      (return (== _asspace_ship _returnvalue)))
    (:`CastFailed`
      (bind _asship_part (cast `/Game/Blueprints/Ship/ShipPart` TestActor)
        (:`then`
          (return (== (`/Game/Blueprints/Ship/ShipPart.OwningShip` _asship_part) _returnvalue)))
        (:`CastFailed`
          (return false))))))

(fn `UserConstructionScript`
  (bind _projectilemovement (`self.ProjectileMovement`))
  (set `ProjectileMovementComponent.InitialSpeed` (+ (`KismetMathLibrary.Dot_VectorVector` (`SceneComponent.GetForwardVector` (`self.Arrow`)) (`self.InheritedVelocity`)) (`ProjectileMovementComponent.InitialSpeed` _projectilemovement)) _projectilemovement)
  (`self.SetLifeSpan` (+ (* (* (`self.InitialLifeSpan`) 0.1) (`KismetMathLibrary.RandomFloatInRange` -1.0 1.0)) (`self.InitialLifeSpan`))))