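; Ship socket item that raises a temporary shield sized to its owning ship, enlarged for each other active shield so they layer.
; TryUse starts it when the cooldown is zero, and a timeline animates the material's Progress before enabling overlaps.
; The cooldown doubles as duration, reversing the animation on expiry.
; Damage drains shield health, and depletion hides it immediately and spawns an explosion in the shield's color.
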(event Custom|StartShield
  (bind _shield (Variables|Default|GetShield))
  (Variables|Default|SetCurrentCooldown (Variables|Default|GetCooldown))
  (Variables|Default|SetCurrentHealth (Variables|Default|GetMaxHealth))
  (Variables|Default|SetIsShieldEnabled true)
  (Rendering|SetVisibility (Variables|Default|GetShield) true false)
  (bind (_direction _progress) (Timeline|ShieldAnim Play)
    (:Update
      (Rendering|Material|SetScalarParameterValue (Variables|Default|GetDMI) "Progress" _progress :!class /Script/Engine.MaterialInstanceDynamic))
    (:Finished
      (switch Utilities|FlowControl|Switch|SwitchonETimelineDirection _direction
        (:Forward
          (Variables|/Script/Engine.PrimitiveComponent|SetbGenerateOverlapEvents _shield true)
          (Development|PrintString "Hello"))
        (:Backward
          (Rendering|SetVisibility _shield false false)
          (Timeline|ShieldAnim SetNewTime))))))

(event Custom|EndShield
  (params (WasDestroyed :type Boolean))
  (bind _shield (Variables|Default|GetShield))
  (Variables|Default|SetCurrentHealth 0.0)
  (Variables|Default|SetIsShieldEnabled false)
  (Variables|/Script/Engine.PrimitiveComponent|SetbGenerateOverlapEvents (Variables|Default|GetShield) false)
  (if WasDestroyed
    (CallFunction|OnDestroy)
    (Rendering|SetVisibility _shield false false :!label _label)
    (bind (_direction _progress) (Timeline|ShieldAnim SetNewTime)
      (:Update
        (Rendering|Material|SetScalarParameterValue (Variables|Default|GetDMI) "Progress" _progress :!class /Script/Engine.MaterialInstanceDynamic))
      (:Finished
        (switch Utilities|FlowControl|Switch|SwitchonETimelineDirection _direction
          (:Forward
            (Variables|/Script/Engine.PrimitiveComponent|SetbGenerateOverlapEvents _shield true)
            (Development|PrintString "Hello"))
          (:Backward
            (goto _label)))))
    (else
      (Timeline|ShieldAnim Reverse))))

(event Game|Damage|EventAnyDamage
  (params (Damage :type Float%20%28single-precision%29) (DamageType :type Damage%20Type%20Object%20Reference) (InstigatedBy :type Controller%20Object%20Reference) (DamageCauser :type Actor%20Object%20Reference))
  (bind _output_get (Variables|Default|SetCurrentHealth (- (Variables|Default|GetCurrentHealth) Damage)))
  (if (<= _output_get 0.0)
    (CallFunction|EndShield true)))

(event EventBeginPlay
  (|CallParentFunction)
  (Transformation|SetWorldLocation (Variables|Default|GetShield) (Transformation|GetWorldLocation (Variables|/Game/Blueprints/Ship/SpaceShip.SpaceShip_C|GetShip (Variables|Default|GetOwningShip))) false false)
  (bind _returnvalue (Rendering|Material|CreateDynamicMaterialInstance (Variables|Default|GetShield) 0 0 :!class /Script/Engine.PrimitiveComponent))
  (Variables|Default|SetDMI _returnvalue))

(event EventActorBeginOverlap
  (params (OtherActor :type Actor%20Object%20Reference)))

(event EventTick
  (params (DeltaSeconds :type Float%20%28single-precision%29))
  (if (> (Variables|Default|GetCurrentCooldown) 0.0)
    (bind _output_get (Variables|Default|SetCurrentCooldown (Math|Float|Clamp(Float) (- (Variables|Default|GetCurrentCooldown) DeltaSeconds) 0.0 (Variables|Default|GetCooldown))))
    (if (== _output_get 0.0)
      (CallFunction|EndShield false))))

(fn ConstructionScript
  (|CallParentFunction)
  (Variables|Default|SetCurrentCooldown (Variables|Default|GetCooldown)))

(fn OnDestroy
  (bind _returnvalue (Rendering|Material|GetVectorParameterValue (Variables|Default|GetDMI) "Color" :!class /Script/Engine.MaterialInstanceDynamic))
  (Game|SpawnActorfromClass "/Game/Blueprints/World/Effects/BurstEffect_ShieldExplosion.BurstEffect_ShieldExplosion_C" (Transformation|GetWorldTransform (Variables|Default|GetShield)) "AlwaysSpawn" 0 (Math|Conversions|ToVector(LinearColor) _returnvalue) 0))

(fn CheckAvailability
  (return true))

(fn CheckReadyforUse
  (return (== (Variables|Default|GetCurrentCooldown) 0.0)))

(fn GetCooldown
  (return (- 1.0 (/ (Variables|Default|GetCurrentCooldown) (Variables|Default|GetCooldown)))))

(fn TryUse
  (bind _isready (CallFunction|CheckReadyforUse))
  (if _isready
    (for _array_element (Variables|/Game/Blueprints/Ship/SpaceShip.SpaceShip_C|GetSocketSlots (Variables|Default|GetOwningShip))
      (Utilities|IsValid (Variables|/Game/Blueprints/Ship/SocketSlot.SocketSlot_C|GetItemInstance _array_element)
        (:Is%20Valid
          (bind _asshield (Utilities|Casting|CastToShield (Variables|/Game/Blueprints/Ship/SocketSlot.SocketSlot_C|GetItemInstance _array_element)))
          (if (Variables|Shield_C|GetIsShieldEnabled _asshield)
            (Math|Integer|IncrementInt (LocalVariables|GetActiveShieldsCount))))))
    (Transformation|SetWorldScale3D (Variables|Default|GetShield) (Math|Conversions|ToVector(Float) (+ (/ (Math|Vector|GetMaxElement (.Max (Components|StaticMesh|GetLocalBounds (Variables|/Game/Blueprints/Ship/SpaceShip.SpaceShip_C|GetShip (Variables|Default|GetOwningShip))))) 35.0) (* (LocalVariables|GetActiveShieldsCount) 0.5))))
    (CallFunction|StartShield)
    (return true)
    (else
      (return false))))