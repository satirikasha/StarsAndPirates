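; Physics-driven spaceship pawn with modular engines and weapons, flown by player input or by an AI controller it spawns when unpossessed.
; Construction builds typed SocketSlots from mesh socket names, and BeginPlay fills engine and weapon slots with default data-table items.
; SpawnItemInSocket attaches item actors and maintains the arrays driven by throttle and fire input.
; Torque handles banked turns and self-levelling, while pickups go to the game mode's inventory manager.
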(event EventBeginPlay
  (CallFunction|SetSocketsDefaultItems)
  (CallFunction|AutoPossessAIController))

(event EventActorBeginOverlap
  (params (OtherActor :type Actor%20Object%20Reference)))

(event EventTick
  (params (DeltaSeconds :type Float%20%28single-precision%29))
  (bind _ship (Variables|Default|GetShip))
  (bind _stabilizationtorque (Variables|Default|GetStabilizationTorque))
  (bind _basearm (Variables|Default|GetBaseArm))
  (bind _returnvalue (Transformation|GetWorldRotation _ship))
  (bind (_roll _pitch) (Math|Rotator|BreakRotator _returnvalue))
  (Class|PrimitiveComponent|AddTorque _ship (+ (* (Math|Vector|GetForwardVector _basearm) (* _roll _stabilizationtorque)) (* (Math|Vector|GetRightVector _basearm) (* _pitch _stabilizationtorque))) "None" false))

(event Input|ActionEvents|InputActionFire
  (params (Key :type Key%20Structure :default "AnyKey"))
  (bind _weapons (Variables|Default|GetWeapons))
  (:Pressed
    (for _array_element _weapons
      (Default|PullTrigger _array_element)))
  (:Released
    (for _array_element_2 _weapons
      (Default|ReleaseTrigger _array_element_2))))

(event Input|AxisEvents|InputAxisThrottle
  (params (AxisValue :type Float%20%28single-precision%29))
  (for _array_element (Variables|Default|GetEngines)
    (Default|RecieveThrottle _array_element AxisValue (Variables|Default|GetShip) (Math|Vector|GetForwardVector (Variables|Default|GetDirection)))))

(event Input|AxisEvents|InputAxisTurn
  (params (AxisValue :type Float%20%28single-precision%29))
  (bind _turntorque (Variables|Default|GetTurnTorque))
  (bind _direction (Variables|Default|GetDirection))
  (Class|PrimitiveComponent|AddTorque (Variables|Default|GetShip) (+ (* (* (Math|Vector|GetUpVector _direction) AxisValue) _turntorque) (* (Math|Vector|GetForwardVector _direction) (* _turntorque AxisValue 0.5 -1.0))) "None" false))

(fn ConstructionScript
  (CallFunction|ConstructSockets))

(fn SetSocketsDefaultItems
  (for _array_element (Variables|Default|GetSocketSlots)
    (switch Utilities|FlowControl|Switch|SwitchonItemType (Variables|/Game/Blueprints/Ship/SocketSlot.SocketSlot_C|GetSocketType _array_element)
      (:NewEnumerator1
        (bind _returnvalue (Utilities|GetDataTableRow "/Game/Blueprints/Data/ItemData.ItemData" "UnionEngine_01")
          (:then
            (Default|SetItem _array_element _returnvalue))))
      (:NewEnumerator2
        (bind _returnvalue_2 (Utilities|GetDataTableRow "/Game/Blueprints/Data/ItemData.ItemData" "UnionWeapon_01")
          (:then
            (Default|SetItem _array_element _returnvalue_2)))))))

(fn GetPlanarVelocity
  (bind _returnvalue (Physics|GetPhysicsLinearVelocity (Variables|Default|GetShip) "None"))
  (return (Math|Vector|MakeVector (.X (Math|Vector|BreakVector _returnvalue)) (.Y (Math|Vector|BreakVector _returnvalue)) 0.0)))

(fn PickUpItem
  (params (Item :type Item%20Container%20Object%20Reference))
  (Default|OnItemPickedUp (CallFunction|GetInventoryManager) (Variables|/Game/Blueprints/Item/ItemContainer.ItemContainer_C|GetItems Item))
  (Actor|DestroyActor Item))

(fn GetInventoryManager
  (Utilities|IsValid (Variables|Default|GetInventoryManager)
    (:Is%20Valid
      (return (Variables|Default|GetInventoryManager)))
    (:Is%20Not%20Valid
      (bind _asflying_game_mode (Utilities|Casting|CastToFlyingGameMode (Game|GetGameMode))
        (:then
          (bind _output_get (Variables|Default|SetInventoryManager (Variables|/Game/Blueprints/FlyingGameMode.FlyingGameMode_C|GetInventoryManager _asflying_game_mode)))
          (return _output_get))
        (:CastFailed
          (return 0))))))

(fn ConstructSockets
  (bind _self self)
  (for _array_element (Transformation|GetAllSocketNames (Variables|Default|GetShip))
    (bind _returnvalue (Game|ConstructObjectfromClass "/Game/Blueprints/Ship/SocketSlot.SocketSlot_C" _self _self _array_element (CallFunction|GetSocketTypefromString (Utilities|Array|Get(acopy) (Utilities|String|ParseIntoArray (Utilities|String|ToString(Name) _array_element) "_" false) 1))))
    (Utilities|Array|Add (Variables|Default|GetSocketSlots) _returnvalue)))

(fn GetSocketTypefromString
  (params (SocketType :type String))
  (bind _enumvalue (|ForEachItemType)
    (:LoopBody
      (if (Utilities|Enum|Equal(Enum) (Utilities|String|EnumtoString _enumvalue) SocketType)
        (LocalVariables|SetResult _enumvalue)))
    (:then
      (return (LocalVariables|GetResult)))))

(fn SpawnIteminSocket
  (params (Item :type Item%20Structure) (Socket :type Socket%20Slot%20Object%20Reference))
  (bind (_itemclass _image _name _description _type) (Utilities|Struct|BreakItem Item))
  (bind _weapons (Variables|Default|GetWeapons))
  (bind _engines (Variables|Default|GetEngines))
  (bind _iteminstance (Variables|/Game/Blueprints/Ship/SocketSlot.SocketSlot_C|GetItemInstance Socket))
  (bind _socketname (Variables|/Game/Blueprints/Ship/SocketSlot.SocketSlot_C|GetSocketName Socket))
  (Utilities|IsValid _iteminstance
    (:Is%20Valid
      (Actor|DestroyActor _iteminstance))
    (:Is%20Not%20Valid
      _))
  (if (Utilities|IsValidClass _itemclass)
    (bind _returnvalue (Game|SpawnActorfromClass _itemclass (Transformation|GetSocketTransform (Variables|Default|GetShip) _socketname "RTS_World") "AlwaysSpawn" self 0))
    (Class|Actor|AttachRootComponentto _returnvalue (Variables|Default|GetShip) _socketname "SnapToTarget" true)
    (switch Utilities|FlowControl|Switch|SwitchonItemType _type
      (:NewEnumerator0
        (return 0))
      (:NewEnumerator1
        (Class|EngineToolsLibrary|RemoveInvalid _engines)
        (Utilities|Array|Add _engines (.AsEngine (Utilities|Casting|CastToEngine _returnvalue))))
      (:NewEnumerator2
        (Class|EngineToolsLibrary|RemoveInvalid _weapons)
        (Utilities|Array|Add _weapons (.AsWeapon (Utilities|Casting|CastToWeapon _returnvalue)))))
    (return _returnvalue)
    (else
      (switch Utilities|FlowControl|Switch|SwitchonItemType (Variables|/Game/Blueprints/Ship/SocketSlot.SocketSlot_C|GetSocketType Socket)
        (:NewEnumerator0
          _)
        (:NewEnumerator1
          (Class|EngineToolsLibrary|RemoveInvalid (Variables|Default|GetEngines)))
        (:NewEnumerator2
          (Class|EngineToolsLibrary|RemoveInvalid (Variables|Default|GetWeapons))))
      (return 0))))

(fn AutoPossessAIController
  (Utilities|IsValid (Pawn|GetController)
    (:Is%20Not%20Valid
      (bind _returnvalue (Game|SpawnActorfromClass (Variables|Default|GetAIControllerClass) (Transformation|GetActorTransform) "Undefined" 0 0))
      (Pawn|Possess _returnvalue self))))