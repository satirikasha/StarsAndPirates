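; A ship socket slot that holds one item tied to a named socket on the ship's mesh.
; SetItem accepts an item when its class validity equals its socket-type match, so invalid, mismatched items also pass, then stores it and keeps the instance its owner spawns.
; GetUniformOffset returns the socket's actor-space X and Y, both divided by the larger X/Y maximum of the ship's local bounds.
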(fn `GetItem`
  (returns (Item :type "/Game/Blueprints/Data/Item Structure"))
  (return (`self.StoredItem`)))

(fn `GetUniformOffset`
  (returns (OffsetX :type "Float (double-precision)") (OffsetY :type "Float (double-precision)"))
  (bind _ship (`/Game/Blueprints/Ship/SpaceShip.Ship` (`self.Owner`)))
  (bind _returnvalue (`KismetMathLibrary.FMax` (.x (`.Max` (`StaticMeshComponent.GetLocalBounds` _ship))) (.y (`.Max` (`StaticMeshComponent.GetLocalBounds` _ship)))))
  (return (/ (.x (.location (`SceneComponent.GetSocketTransform` _ship (`self.SocketName`) "RTS_Actor"))) _returnvalue) (/ (.y (.location (`SceneComponent.GetSocketTransform` _ship (`self.SocketName`) "RTS_Actor"))) _returnvalue)))

(fn `SetItem`
  (params (Item :type "/Game/Blueprints/Data/Item Structure"))
  (bind (_itemclass _image _name _description _type) (break `/Game/Blueprints/Data/Item` Item))
  (if (== (`KismetSystemLibrary.IsValidClass` _itemclass) (`|EnumEquality` _type (`self.SocketType`)))
    (bind _output_get (set `self.StoredItem` Item))
    (bind _iteminstance (`/Game/Blueprints/Ship/SpaceShip.SpawnItemInSocket` (`self.Owner`) _output_get self (`self.Visibility`)))
    (set `self.ItemInstance` _iteminstance)))