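; FlyingGameMode is the game mode for the space flying level, using SpaceShip as the default pawn for every controller.
; On BeginPlay it spawns the gameplay managers at the origin and keeps references to the segment provider, space object provider, inventory manager and world generation manager.
; It also spawns a WS_Random segment at world cell 0,0 and passes it to WorldGenerationManager as the initial world segment.
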(event `self.ReceiveBeginPlay`
  (bind _returnvalue (`KismetMathLibrary.MakeTransform` (0.0 0.0 0.0)))
  (bind _returnvalue_2 (`|SpawnActorFromClass` "/Game/Blueprints/World/SegmentProvider.SegmentProvider_C" _returnvalue "Undefined" "OverrideRootScale"))
  (set `self.SegmentProvider` _returnvalue_2)
  (bind _returnvalue_3 (`|SpawnActorFromClass` "/Game/Blueprints/World/SpaceObjectProvider.SpaceObjectProvider_C" _returnvalue "Undefined" "OverrideRootScale"))
  (set `self.SpaceObjectProvider` _returnvalue_3)
  (bind _returnvalue_4 (`|SpawnActorFromClass` "/Game/Blueprints/World/Item/InventoryManager.InventoryManager_C" _returnvalue "Undefined" "OverrideRootScale"))
  (set `self.InventoryManager` _returnvalue_4)
  (bind _returnvalue_5 (`|SpawnActorFromClass` "/Game/Blueprints/World/Segments/WS_Random.WS_Random_C" _returnvalue "Undefined" "OverrideRootScale"))
  (bind _returnvalue_6 (`|SpawnActorFromClass` "/Game/Blueprints/World/WorldGenerationManager.WorldGenerationManager_C" _returnvalue "Undefined" "OverrideRootScale" null _returnvalue_5))
  (set `self.WorldGenerationManager` _returnvalue_6))

(event `self.ReceiveTick`
  (params (DeltaSeconds :type "Float (single-precision)")))

(fn `GetDefaultPawnClassForController`
  (params (InController :type "Controller Object Reference"))
  (returns (ReturnValue :type "Object Class Reference"))
  (return "/Game/Blueprints/Ship/SpaceShip.SpaceShip_C"))

(fn `UserConstructionScript`)